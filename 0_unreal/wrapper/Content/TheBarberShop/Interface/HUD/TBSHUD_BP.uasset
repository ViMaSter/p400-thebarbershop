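; Main HUD for The Barber Shop that creates the game's menu, stats, tool, shop, editor and other screen widgets at BeginPlay, starting in the Intro state.
; Tick updates the level text, an experience-filled barber pole material and the clock, which holds while paused.
; Input events drive beard undo/redo and switch StateComponent between editor and pause states.
; Helper functions route beard load, save and delete requests to the editor's confirmation dialogs.
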(event Custom|LaunchMenu
  ;[1 1 1] Open menu
  (bind _astbsplayer_controller (Utilities|Casting|CastToTBSPlayerController (Game|GetPlayerController 0)))
  (Variables|/Script/Engine.PlayerController|SetbShowMouseCursor _astbsplayer_controller true)
  (Class|TBSPlayerController|SetIsIngame _astbsplayer_controller false)
  (Class|StateComponent|SettoState (Variables|Default|GetStateComponent) (Utilities|Enum|LiteralenumETBSHUDState "MainMenu")))

(event EventBeginPlay
  (Class|StateComponent|SettoState (Variables|Default|GetStateComponent) (Utilities|Enum|LiteralenumETBSHUDState "Intro"))
  (Input|EnableInput (Game|GetPlayerController 0))
  (Utilities|FlowControl|Sequence
    (:then_0
      (bind _returnvalue (UserInterface|CreateWidget "/Game/TheBarberShop/Interface/HUD/Ingame/PauseMenu/Ingame_PauseMenu.Ingame_PauseMenu_C"))
      (bind _output_get (Variables|Default|SetIngame_PauseMenu _returnvalue))
      (UserInterface|Viewport|AddtoViewport _output_get 0))
    (:then_1
      (bind _returnvalue_2 (UserInterface|CreateWidget "/Game/TheBarberShop/Interface/HUD/Options/Options_Menu.Options_Menu_C"))
      (bind _output_get_2 (Variables|Default|SetOptions _returnvalue_2))
      (UserInterface|Viewport|AddtoViewport _output_get_2 0))
    (:then_2
      (bind _returnvalue_3 (UserInterface|CreateWidget "/Game/TheBarberShop/Interface/HUD/Options/Options_Audio.Options_Audio_C"))
      (bind _output_get_3 (Variables|Default|SetOptions_Audio _returnvalue_3))
      (UserInterface|Viewport|AddtoViewport _output_get_3 0))
    (:then_3
      (bind _returnvalue_4 (UserInterface|CreateWidget "/Game/TheBarberShop/Interface/HUD/Options/Options_Video.Options_Video_C"))
      (bind _output_get_4 (Variables|Default|SetOptions_Video _returnvalue_4))
      (UserInterface|Viewport|AddtoViewport _output_get_4 0))
    (:then_4
      (bind _returnvalue_5 (UserInterface|CreateWidget "/Game/TheBarberShop/Interface/HUD/Ingame/Stats/Stats.Stats_C"))
      (bind _output_get_5 (Variables|Default|SetIngame_Stats _returnvalue_5))
      (UserInterface|Viewport|AddtoViewport _output_get_5 0))
    (:then_5
      (bind _returnvalue_6 (UserInterface|CreateWidget "/Game/TheBarberShop/Interface/HUD/Ingame/ToolBar/ToolBar.ToolBar_C"))
      (bind _output_get_6 (Variables|Default|SetIngame_Tools _returnvalue_6))
      (UserInterface|Viewport|AddtoViewport _output_get_6 0))
    (:then_6
      (bind _returnvalue_7 (UserInterface|CreateWidget "/Game/TheBarberShop/Interface/HUD/Ingame/EditorInterface/EditorInterface.EditorInterface_C"))
      (bind _output_get_7 (Variables|Default|SetEditor _returnvalue_7))
      (UserInterface|Viewport|AddtoViewport _output_get_7 0))
    (:then_7
      (bind _returnvalue_8 (UserInterface|CreateWidget "/Game/TheBarberShop/Interface/HUD/Ingame/ResultScreen/ResultScreen.ResultScreen_C"))
      (bind _output_get_8 (Variables|Default|SetResultScreen _returnvalue_8))
      (UserInterface|Viewport|AddtoViewport _output_get_8 0))
    (:then_8
      (bind _returnvalue_9 (UserInterface|CreateWidget "/Game/TheBarberShop/Interface/HUD/Ingame/Shop/ShopMain.ShopMain_C"))
      (bind _output_get_9 (Variables|Default|SetShop _returnvalue_9))
      (UserInterface|Viewport|AddtoViewport _output_get_9 0))
    (:then_9
      (bind _returnvalue_10 (UserInterface|CreateWidget "/Game/TheBarberShop/Interface/HUD/Ingame/BeardManager/BeardMain.BeardMain_C"))
      (bind _output_get_10 (Variables|Default|SetBeardOverview _returnvalue_10))
      (UserInterface|Viewport|AddtoViewport _output_get_10 0))
    (:then_11
      (bind _returnvalue_11 (UserInterface|CreateWidget "/Game/TheBarberShop/Interface/HUD/StartScreen/StartScreen_GamesAcademy.StartScreen_GamesAcademy_C"))
      (bind _output_get_11 (Variables|Default|SetStartScreen_GamesAcademy _returnvalue_11))
      (UserInterface|Viewport|AddtoViewport _output_get_11 0))
    (:then_12
      (bind _returnvalue_12 (UserInterface|CreateWidget "/Game/TheBarberShop/Interface/HUD/Ingame/Radio/Radio.Radio_C"))
      (bind _output_get_12 (Variables|Default|SetRadio _returnvalue_12))
      (UserInterface|Viewport|AddtoViewport _output_get_12 0))))

(event EventTick
  (params (DeltaSeconds :type Float%20%28single-precision%29))
  (Utilities|FlowControl|Sequence
    (:then_0
      ;[1 1 1] Barber pole material example
      (bind _astbscharacter (Utilities|Casting|CastToTBSCharacter (Class|HUD|GetOwningPawn)))
      (Rendering|Material|SetScalarParameterValue (Variables|/Game/TheBarberShop/Interface/HUD/Ingame/Stats/Stats.Stats_C|GetBarberPole_pole_instance (Variables|Default|GetIngame_Stats)) "PercentageFilled" (* (/ (Math|Conversions|ToFloat(Integer) (Variables|/Script/TBS.TBSCharacter|GetCurrentExperience _astbscharacter)) (Math|Conversions|ToFloat(Integer) (Variables|/Script/TBS.TBSCharacter|GetCurrentExperienceToLvl _astbscharacter))) 1e+02) :!class /Script/Engine.MaterialInstanceDynamic))
    (:then_1
      ;[1 1 1] Barber pole material example
      (bind _astbscharacter_2 (Utilities|Casting|CastToTBSCharacter (Class|HUD|GetOwningPawn)))
      (Rendering|Components|TextRender|SetText (Variables|/Game/TheBarberShop/Interface/HUD/Ingame/Stats/Stats.Stats_C|GetCurrentLevel (Variables|Default|GetIngame_Stats)) (Utilities|Text|ToText(Integer) (+ (Variables|/Script/TBS.TBSCharacter|GetCurrentLevel _astbscharacter_2) 1) true 2 2)))
    (:then_2
      ;[1 1 1] Update Clock
      (bind _astbsgame_state_bp (Utilities|Casting|CastToTBSGameState_BP (Game|GetGameState)))
      (bind _returnvalue (Class|TBSGameState|GetIsPaused _astbsgame_state_bp))
      (if (not _returnvalue)
        (bind _astbscharacter_3 (Utilities|Casting|CastToTBSCharacter (Class|HUD|GetOwningPawn)))
        (bind _returnvalue_2 (Class|TBSCharacter|GetTimeElapsed _astbscharacter_3))
        (Default|UpdateClock (Variables|Default|GetIngame_Stats) (Math|Conversions|ToFloat(Integer) (Math|Float|Floor (/ _returnvalue_2 6e+01))) (Math|Float|%(Float) _returnvalue_2 6e+01))))))

(event Input|ActionEvents|InputActionUI_PauseMenu
  ;[1 1 1] HUD-toggling
  (:Pressed
    (Class|StateComponent|SettoState (Variables|Default|GetStateComponent) (Utilities|Enum|LiteralenumETBSHUDState "PauseMenu"))
    (bind _astbsplayer_controller (Utilities|Casting|CastToTBSPlayerController (Game|GetPlayerController 0)))
    (Variables|/Script/Engine.PlayerController|SetbShowMouseCursor _astbsplayer_controller true)
    (Class|TBSPlayerController|SetIsIngame _astbsplayer_controller false)
    (Class|TBSPlayerController|SetIsPaused _astbsplayer_controller true)))

(event Input|ActionEvents|InputActionUndoLastChange
  ;[1 1 1] Bind beard-history-functions to keys
  (:Pressed
    (bind _astbsplayer_controller_bp (Utilities|Casting|CastToTBSPlayerController_BP (Game|GetPlayerController 0)))
    (Class|TBSPlayerController|UndoBeardChanges _astbsplayer_controller_bp)))

(event Input|ActionEvents|InputActionRedoLastChange
  ;[1 1 1] Bind beard-history-functions to keys
  (:Pressed
    (bind _astbsplayer_controller_bp (Utilities|Casting|CastToTBSPlayerController_BP (Game|GetPlayerController 0)))
    (Class|TBSPlayerController|RedoBeardChanges _astbsplayer_controller_bp)))

(event Input|ActionEvents|InputActionUI_EditorMenu
  ;[1 1 1] HUD-toggling
  (:Pressed
    (bind _astbsplayer_controller (Utilities|Casting|CastToTBSPlayerController (Game|GetPlayerController 0)))
    (bind _returnvalue (Class|TBSPlayerController|GetIsEditorMode _astbsplayer_controller))
    (if _returnvalue
      (bind _aseditor_interface (Utilities|Casting|CastToEditorInterface (Variables|Default|GetEditor)))
      (Default|RefreshList _aseditor_interface)
      (Class|StateComponent|ToggleState (Variables|Default|GetStateComponent) (Utilities|Enum|LiteralenumETBSHUDState "EditorDialogue")))))

(fn ConstructionScript)

(fn TryLoadBeard
  (params (BeardName :type Name :default "None"))
  ;[1 1 1] Check whether or not the beard exists
  (bind _astbsplayer_controller (Utilities|Casting|CastToTBSPlayerController (Game|GetPlayerController 0)))
  (bind _returnvalue (Class|TBSPlayerController|GetBeardNameLevelData _astbsplayer_controller))
  (bind _array_element (Utilities|Array|ForEachLoopwithBreak _returnvalue :!label _label)
    (:LoopBody
      (if (Utilities|Name|Equal(Name) (.BeardName (Utilities|Struct|BreakBeardNameLevelData _array_element)) BeardName)
        (LocalVariables|SetisSuccess true)
        (goto _label Break)))
    (:Completed
      (if (LocalVariables|GetisSuccess)
        ;[1 1 1] Open Confirmation-Dialog if so
        (bind _aseditor_interface (Utilities|Casting|CastToEditorInterface (Variables|Default|GetEditor)))
        (Default|ChangeBeardtoLoad _aseditor_interface BeardName false))
      (return (LocalVariables|GetisSuccess)))))

(fn TrySaveBeard
  (params (BeardName :type Name :default "None"))
  ;[1 1 1] Open Confirmation-Dialog if so
  (bind _aseditor_interface (Utilities|Casting|CastToEditorInterface (Variables|Default|GetEditor)))
  (Default|ChangeBeardtoSave _aseditor_interface BeardName false))

(fn TryDeleteBeard
  (params (BeardName :type Name :default "None"))
  ;[1 1 1] Open Confirmation-Dialog if so
  (bind _aseditor_interface (Utilities|Casting|CastToEditorInterface (Variables|Default|GetEditor)))
  (Default|ChangeBeardtoDelete _aseditor_interface BeardName false))