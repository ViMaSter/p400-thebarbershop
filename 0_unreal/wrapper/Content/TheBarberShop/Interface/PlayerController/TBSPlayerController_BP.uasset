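; Player controller for a barber shop game that handles customer transitions, saving and menu input.
; On BeginPlay it attaches the audio listener to the character's camera and loads the game.
; Finishing a customer outside editor mode shows beard results with a render-target comparison image and saves, then the shop always reloads.
; Spawning the next customer resets results, repositions the pause-menu plate and runs a cutscene; input drives editor, pause and undo/redo.
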(event EventSpawnedNextCustomer
  ;[0.145 0.02175 0.02175] Events
  (Utilities|FlowControl|Sequence
    (:then_0
      (bind _astbshud_bp (Utilities|Casting|CastToTBSHUD_BP (HUD|GetHUD)))
      (bind _asresult_screen (Utilities|Casting|CastToResultScreen (Variables|/Game/TheBarberShop/Interface/HUD/TBSHUD_BP.TBSHUD_BP_C|GetResultScreen _astbshud_bp)))
      (Variables|/Game/TheBarberShop/Interface/HUD/Ingame/ResultScreen/ResultScreen.ResultScreen_C|SetFloatPercentageTarget _asresult_screen 0.0)
      (bind _ascharacter_bp (Utilities|Casting|CastToCharacter_BP (Pawn|GetControlledPawn)))
      (Transformation|SetActorLocation (Variables|/Game/TheBarberShop/Interface/HUD/TBSHUD_BP.TBSHUD_BP_C|GetPauseMenuPlate _astbshud_bp) (select (Variables|/Script/TBS.TBSCharacter|GetFirstCustomerActive _ascharacter_bp) "55.000000,-810.000000,340.000000" "55.000000,0.000000,340.000000") false))
    (:then_1
      (bind _astbscharacter (Utilities|Casting|CastToTBSCharacter (Pawn|GetControlledPawn)))
      (Default|CallRunCutscene "NewEnumerator0" false (Variables|/Script/TBS.TBSCharacter|GetFirstCustomerActive _astbscharacter)))))

(event EventFinishedCurrentCustomer
  ;[0.145 0.02175 0.02175] Events
  (Utilities|FlowControl|Sequence
    (:then_0
      ;;[1 1 1] Show result screen, if we're in play-mode
      (bind _returnvalue (Class|TBSPlayerController|GetIsEditorMode))
      (if (not _returnvalue)
        (bind _astbshud (Utilities|Casting|CastToTBSHUD (HUD|GetHUD)))
        (Class|StateComponent|SetState (Variables|/Script/TBS.TBSHUD|GetStateComponent _astbshud) (Utilities|Enum|LiteralenumETBSHUDState "Results") true)
        (Variables|Default|SetbShowMouseCursor true)
        (Utilities|FlowControl|Sequence
          (:then_0
            ;;[1 1 1] Queue interface animation
            (bind _astbshud_bp (Utilities|Casting|CastToTBSHUD_BP (HUD|GetHUD)))
            (bind _asresult_screen (Utilities|Casting|CastToResultScreen (Variables|/Game/TheBarberShop/Interface/HUD/TBSHUD_BP.TBSHUD_BP_C|GetResultScreen _astbshud_bp)))
            (bind _astbscharacter (Utilities|Casting|CastToTBSCharacter (Pawn|GetControlledPawn)))
            (bind _returnvalue_2 (Class|TBSCharacter|GetTimeElapsed _astbscharacter))
            (Default|UpdateValues _asresult_screen (Variables|/Script/TBS.TBSCharacter|GetLastBeardResult _astbscharacter) _returnvalue_2)
            (Utilities|FlowControl|Delay 0 1.0)
            (Variables|/Game/TheBarberShop/Interface/HUD/Ingame/ResultScreen/ResultScreen.ResultScreen_C|SetFloatPercentageTarget _asresult_screen (Variables|/Script/TBS.TBSCharacter|GetLastBeardResult _astbscharacter))
            (Development|PrintString 0 (Utilities|String|ToString(Float) (Variables|/Script/TBS.TBSCharacter|GetLastBeardResult _astbscharacter))))
          (:then_1
            ;;[1 1 1] Save game
            (bind _astbsgame_state_bp (Utilities|Casting|CastToTBSGameState_BP (Game|GetGameState)))
            (Class|TBSGameState|SaveGame _astbsgame_state_bp))
          (:then_2
            ;;[1 1 1] Set currently shaved beard image
            (bind _astbscharacter_2 (Utilities|Casting|CastToTBSCharacter (Pawn|GetControlledPawn)))
            (bind _ascustomer_bp (Utilities|Casting|CastToCustomer_BP (Variables|/Script/TBS.TBSCharacter|GetCurrentCustomer _astbscharacter_2)))
            (Class|SceneCaptureComponent2D|UpdateContent (Variables|/Script/TBS.TBSCustomer|GetSceneCapture _ascustomer_bp)))
          (:then_3
            ;;[1 1 1] Set original beard image
            (bind _astbscharacter_3 (Utilities|Casting|CastToTBSCharacter (Pawn|GetControlledPawn)))
            (bind _astbshud_bp_2 (Utilities|Casting|CastToTBSHUD_BP (HUD|GetHUD)))
            (bind _asresult_screen_2 (Utilities|Casting|CastToResultScreen (Variables|/Game/TheBarberShop/Interface/HUD/TBSHUD_BP.TBSHUD_BP_C|GetResultScreen _astbshud_bp_2)))
            (bind _returnvalue_3 (Rendering|Material|CreateDynamicMaterialInstance 0 "/Game/TheBarberShop/Data/BeardIconUIMaterial.BeardIconUIMaterial" :!class /Script/Engine.KismetMaterialLibrary))
            (Rendering|Material|SetTextureParameterValue _returnvalue_3 "RenderTarget" (.ComparisionScreenshot (Utilities|Struct|BreakBeardCollectionData (Variables|/Script/TBS.TBSCharacter|GetCurrentBeardRow _astbscharacter_3))))
            (Class|Image|SetBrushfromMaterial (Variables|/Game/TheBarberShop/Interface/HUD/Ingame/ResultScreen/ResultScreen.ResultScreen_C|GetLeftBoxImage _asresult_screen_2) _returnvalue_3)))))
    (:then_1
      ;;[1 1 1] Update shop (since we load the vaules using multithreadding)
      (bind _astbshud_bp_3 (Utilities|Casting|CastToTBSHUD_BP (HUD|GetHUD)))
      (Default|ReloadStoreItems (Variables|/Game/TheBarberShop/Interface/HUD/TBSHUD_BP.TBSHUD_BP_C|GetShop _astbshud_bp_3)))))

(event EventBeginPlay
  (bind _self self)
  ;[0.145 0.02175 0.02175] Events
  ;;[1 1 1] Prepare input
  (Input|EnableInput _self _self)
  (bind _astbscharacter (Utilities|Casting|CastToTBSCharacter (Pawn|GetControlledPawn)))
  ;;[1 1 1] Prepare audio
  (Class|PlayerController|SetAudioListenerOverride (Variables|/Script/TBS.TBSCharacter|GetCameraComponent _astbscharacter) "0, 0, 0" "0, 0, 0")
  ;;[1 1 1] Load game
  (bind _astbsgame_state_bp (Utilities|Casting|CastToTBSGameState_BP (Game|GetGameState)))
  (Class|TBSGameState|LoadGame _astbsgame_state_bp))

(event Input|ActionEvents|InputActionUI_PauseMenu
  ;[0.01608 0.01888 0.275] Input mappings
  ;;[1 1 1] Ingame HUD toggles
  (:Pressed
    (bind _astbshud_bp (Utilities|Casting|CastToTBSHUD_BP (HUD|GetHUD)))
    (Class|StateComponent|SettoState (Variables|/Script/TBS.TBSHUD|GetStateComponent _astbshud_bp) (Utilities|Enum|LiteralenumETBSHUDState "PauseMenu"))
    (bind _astbsplayer_controller (Utilities|Casting|CastToTBSPlayerController (Game|GetPlayerController 0)))
    (Variables|/Script/Engine.PlayerController|SetbShowMouseCursor _astbsplayer_controller true)
    (Class|TBSPlayerController|SetIsIngame _astbsplayer_controller false)
    (Class|TBSPlayerController|SetIsPaused _astbsplayer_controller true)))

(event Input|ActionEvents|InputActionUndoLastChange
  ;[0.01608 0.01888 0.275] Input mappings
  ;;[0.035 0.035 0.035] Editor redo/undo
  (:Pressed
    (Class|TBSPlayerController|UndoBeardChanges)))

(event Input|ActionEvents|InputActionRedoLastChange
  ;[0.01608 0.01888 0.275] Input mappings
  ;;[0.035 0.035 0.035] Editor redo/undo
  (:Pressed
    (Class|TBSPlayerController|RedoBeardChanges)))

(event Input|ActionEvents|InputActionUI_EditorMenu
  ;[0.01608 0.01888 0.275] Input mappings
  ;;[1 1 1] Ingame HUD toggles
  (:Pressed
    (bind _astbshud_bp (Utilities|Casting|CastToTBSHUD_BP (HUD|GetHUD)))
    (bind _returnvalue (Class|TBSPlayerController|GetIsEditorMode))
    (if _returnvalue
      (bind _aseditor_interface (Utilities|Casting|CastToEditorInterface (Variables|/Game/TheBarberShop/Interface/HUD/TBSHUD_BP.TBSHUD_BP_C|GetEditor _astbshud_bp)))
      (Default|RefreshList _aseditor_interface)
      (Class|StateComponent|ToggleState (Variables|/Script/TBS.TBSHUD|GetStateComponent _astbshud_bp) (Utilities|Enum|LiteralenumETBSHUDState "EditorDialogue")))))

(fn ConstructionScript)