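; Beard style actor for The Barber Shop that builds a customer's beard from individual hair meshes.
; The construction script reads hair transforms from the BeardStyle_00 data table, adding either instances or separate static mesh components set to ignore Camera and use Destructible collision.
; When AnimateBeard is on, Tick rotates the actor with the owning current customer's head socket, using fixed angle offsets.
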(event EventTick
  (params (DeltaSeconds :type Float%20%28single-precision%29))
  (if (Variables|Default|GetbAnimateBeard)
    (bind _ascustomer_bp (Utilities|Casting|CastToCustomer_BP (Components|GetOwner)))
    (if (Variables|/Script/TBS.TBSCustomer|GetIsCurrentCustomer _ascustomer_bp)
      (Transformation|SetActorRotation (Class|KismetMathLibrary|MakeRot (+ (.Pitch (Class|KismetMathLibrary|BreakRot (Transformation|GetSocketRotation (Variables|/Game/TheBarberShop/Assets/Customer_BP.Customer_BP_C|GetSkeletalMesh _ascustomer_bp) "head"))) -3e+01) (.Yaw (Class|KismetMathLibrary|BreakRot (Transformation|GetSocketRotation (Variables|/Game/TheBarberShop/Assets/Customer_BP.Customer_BP_C|GetSkeletalMesh _ascustomer_bp) "head"))) (- (.Roll (Class|KismetMathLibrary|BreakRot (Transformation|GetSocketRotation (Variables|/Game/TheBarberShop/Assets/Customer_BP.Customer_BP_C|GetSkeletalMesh _ascustomer_bp) "head"))) 9e+01))))))

(fn ConstructionScript
  (bind _outrownames (DataTable|GetDataTableRowNames "/Game/TheBarberShop/Assets/Characters/BeardStyles/BeardStyle_00.BeardStyle_00"))
  (for _array_element _outrownames
    (bind _returnvalue (Utilities|GetDataTableRow "/Game/TheBarberShop/Assets/Characters/BeardStyles/BeardStyle_00.BeardStyle_00" _array_element)
      (:then
        (if (Variables|Default|GetbUseInstancedMeshes)
          (Components|InstancedStaticMesh|AddInstance (Variables|Default|GetBeardHairInstances) (|Data->Transform _returnvalue))
          (else
            (bind _returnvalue_2 (AddComponent|AddStaticMeshComponent false (|Data->Transform _returnvalue)))
            (Utilities|FlowControl|Sequence
              (:then_0
                (Components|StaticMesh|SetStaticMesh _returnvalue_2 "/Game/TheBarberShop/Assets/Characters/BeardStyles/BeardHair_00.BeardHair_00"))
              (:then_1
                (Rendering|Material|SetMaterial _returnvalue_2 0 "/Game/TheBarberShop/Assets/Characters/MI_Char_01_Beard.MI_Char_01_Beard"))
              (:then_2
                (Collision|SetCollisionResponsetoChannel _returnvalue_2 "ECC_Camera" "ECR_Ignore"))
              (:then_3
                (Collision|SetCollisionObjectType _returnvalue_2 "ECC_Destructible")))))))))