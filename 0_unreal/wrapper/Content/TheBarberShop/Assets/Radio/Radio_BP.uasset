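; Radio Blueprint for the barber shop game that lets the player switch stations and shows the current song on the HUD.
; It enables input from the first player controller at BeginPlay, and the R key calls SwitchStation.
; When the song changes, it passes the new artist and title to the Radio element of TBSHUD_BP.
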(event EventBeginPlay
  (Input|EnableInput (Game|GetPlayerController 0)))

(event EventOnSongChange
  (params (NewSong :type TBS%20Radio%20Song%20Structure))
  (bind (_artist _title) (Utilities|Struct|BreakTBSRadioSong NewSong))
  (bind _returnvalue (Game|GetPlayerController 0))
  (Utilities|IsValid _returnvalue
    (:Is%20Valid
      (bind _astbshud_bp (Utilities|Casting|CastToTBSHUD_BP (HUD|GetHUD _returnvalue)))
      (Default|UpdateRadio (Variables|/Game/TheBarberShop/Interface/HUD/TBSHUD_BP.TBSHUD_BP_C|GetRadio _astbshud_bp) _artist _title))))

(event Input|KeyboardEvents|R
  (:Pressed
    (Class|TBSRadio|SwitchStation 1)))

(fn ConstructionScript)