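; Customer Blueprint for the barber shop game that starts a looping idle skeletal animation once it is the current customer.
; If head animation is enabled on BeginPlay, a short non-looping timer re-arms itself to poll the current-customer flag until it can play the idle.
; An unconnected chain would reset the beard's static meshes to visible, overlap collision and zero trim on their dynamic materials, but never runs.
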(event Custom|PlayAnimation
  (if (Variables|Default|GetIsCurrentCustomer)
    (Components|Animation|PlayAnimation (Variables|Default|GetSkeletalMesh) "/Game/TheBarberShop/Assets/Characters/animtest/Char_Anim_Idle_01.Char_Anim_Idle_01" true)
    (else
      (Utilities|Time|SetTimerbyEvent (delegate Custom|PlayAnimation) 0.1))))

(event EventBeginPlay
  (if (Variables|Default|GetAnimateHead)
    (Utilities|Time|SetTimerbyEvent (delegate Custom|PlayAnimation) 0.1)))

(fn ConstructionScript)