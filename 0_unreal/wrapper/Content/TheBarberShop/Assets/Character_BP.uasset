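; Character Blueprint for the barber shop game that applies equipped item skins to its barber tool.
; The EquipedItem event casts the Tool reference to Tool_BP and uses the item ID to assign a silver clipper, small razor or large razor mesh.
; It then refreshes the tool's Razor static mesh component with the stored mesh matching the current ToolType.
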(event EventEquipedItem
  (params (ID :type Integer))
  (bind _astool_bp (Utilities|Casting|CastToTool_BP (Variables|Default|GetTool)))
  (switch int ID
    (:0
      (bind _output_get (Variables|/Game/TheBarberShop/Assets/Tool_BP.Tool_BP_C|SetClipperMesh _astool_bp "/Game/TheBarberShop/Assets/Clipper/SilverClipper/SilverClipper.SilverClipper")))
    (:1
      (bind _output_get_2 (Variables|/Game/TheBarberShop/Assets/Tool_BP.Tool_BP_C|SetRazorSmallMesh _astool_bp "/Game/TheBarberShop/Assets/RazorSmall/SilverRazor/SilverRazor_S.SilverRazor_S")))
    (:2
      (bind _output_get_3 (Variables|/Game/TheBarberShop/Assets/Tool_BP.Tool_BP_C|SetRazorMesh _astool_bp "/Game/TheBarberShop/Assets/Razor/SilverRazor/SilverRazor_L.SilverRazor_L"))))
  (switch Utilities|FlowControl|Switch|SwitchonETBSRazor (Variables|/Script/TBS.TBSRazor|GetToolType _astool_bp)
    (:TBSClipper
      (Components|StaticMesh|SetStaticMesh (Variables|/Game/TheBarberShop/Assets/Tool_BP.Tool_BP_C|GetRazor _astool_bp) _output_get))
    (:TBSRazorSmall
      (Components|StaticMesh|SetStaticMesh (Variables|/Game/TheBarberShop/Assets/Tool_BP.Tool_BP_C|GetRazor _astool_bp) _output_get_2))
    (:TBSRazorBig
      (Components|StaticMesh|SetStaticMesh (Variables|/Game/TheBarberShop/Assets/Tool_BP.Tool_BP_C|GetRazor _astool_bp) _output_get_3))))

(fn ConstructionScript)