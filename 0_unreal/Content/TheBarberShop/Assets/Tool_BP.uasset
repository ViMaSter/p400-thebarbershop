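; Barber tool actor for The Barber Shop that cuts beard hair on overlap and swaps its Razor mesh when the tool type changes.
; While active, one tool type trims hair through a "Trim%" dynamic material parameter and others hide it, spawning hair particles and flagging the controller's beard as changed.
; Collision channels separate the clipper from other tools, so trimmed hair ignores the clipper's channel.
; The surface-normal rotation logic is mostly disconnected.
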(event OnComponentBeginOverlap(Razor)
  (params (OtherActor :type Actor%20Object%20Reference) (OtherComp :type Primitive%20Component%20Object%20Reference) (OtherBodyIndex :type Integer) (bFromSweep :type Boolean) (SweepResult :type Hit%20Result%20Structure%20%28by%20ref%29))
  (bind _returnvalue (Transformation|GetActorLocation))
  ;[1 1 1] Shave + Particles
  (if (Variables|Default|GetIsActive)
    (bind _asstatic_mesh_component (Utilities|Casting|CastToStaticMeshComponent OtherComp))
    (if (== (Variables|Default|GetToolType) 1)
      (CallFunction|TrimBeardHair _asstatic_mesh_component 0.8)
      (bind _returnvalue_2 (Effects|SpawnEmitteratLocation 0 "/Game/TheBarberShop/Assets/VFX/HairFling_CPU.HairFling_CPU" _returnvalue (Transformation|GetWorldRotation _asstatic_mesh_component)))
      (Transformation|SetWorldScale3D _returnvalue_2 "0.500000,0.500000,0.500000")
      (else
        ;;[1 1 1] Cut
        (Rendering|SetVisibility _asstatic_mesh_component false false)
        (Collision|SetCollisionResponsetoAllChannels _asstatic_mesh_component "ECR_Ignore")
        (bind _returnvalue_3 (Effects|SpawnEmitteratLocation 0 "/Game/TheBarberShop/Assets/VFX/HairFling_CPU.HairFling_CPU" _returnvalue (Transformation|GetWorldRotation _asstatic_mesh_component)))
        (Utilities|Casting|CastToMaterialInstanceDynamic (Rendering|Material|GetMaterial _asstatic_mesh_component 0))
        (Transformation|SetWorldScale3D _returnvalue_3 "0.500000,0.500000,0.500000")))
    ;[1 1 1] Set Changed Beard Bool for Saving the Beard in Editormode
    (bind _astbsplayer_controller_bp (Utilities|Casting|CastToTBSPlayerController_BP (Game|GetPlayerController 0)))
    (Class|TBSPlayerController|SetChangedBeard _astbsplayer_controller_bp)))

(event Custom|CustomEvent_0
  (bind _razor (Variables|Default|GetRazor))
  (bind _returnvalue (Transformation|GetWorldTransform _razor))
  (bind (_location _rotation _scale) (Math|Transform|BreakTransform _returnvalue))
  ;[1 1 1] Rotation Based on Surface Normal
  (Variables|Default|SetTransformBuffer (Math|Transform|MakeTransform _location (stale _output_get) _scale))
  (Utilities|Time|SetTimerbyEvent (delegate Custom|CustomEvent_1) 1.0))

(event Custom|CustomEvent_1
  (bind _razor (Variables|Default|GetRazor))
  (bind _returnvalue (Transformation|GetWorldTransform _razor))
  (bind (_location _rotation _scale) (Math|Transform|BreakTransform _returnvalue))
  ;[1 1 1] Rotation Based on Surface Normal
  (Variables|Default|SetTransformUpdate (Math|Transform|MakeTransform _location (stale _output_get) _scale))
  (Timeline|Timeline_0 PlayFromStart
    (:Update
      (Transformation|SetWorldRotation _razor (* (.Rotation (Math|Transform|BreakTransform (Class|KismetMathLibrary|TInterpto (Variables|Default|GetTransformBuffer) (Variables|Default|GetTransformUpdate) (stale EventTick DeltaSeconds) 0.5))) 1.0) false))))

(event EventTick
  (params (DeltaSeconds :type Float%20%28single-precision%29))
  ;[1 1 1] Rotation Based on Surface Normal
)

(event EventTrimmed
  (params (TrimmValue :type Float%20%28single-precision%29) (Mesh :type Actor%20Component%20Object%20Reference))
  ;[1 1 1] Shave + Particles
  (bind _asstatic_mesh_component (Utilities|Casting|CastToStaticMeshComponent Mesh))
  (CallFunction|TrimBeardHair _asstatic_mesh_component TrimmValue))

(event EventBeginPlay
  ;[1 1 1] Rotation Based on Surface Normal
)

(event EventSwitchedTool
  (params (NewToolType :type ETBSRazor%20Enum :default "TBSHand"))
  ;[1 1 1] Handle Meshes
  (Components|StaticMesh|SetStaticMesh (Variables|Default|GetRazor) (Utilities|Select :Index NewToolType :TBSHand (Variables|Default|GetHandMesh) :TBSClipper (Variables|Default|GetClipperMesh) :TBSRazorSmall (Variables|Default|GetRazorSmallMesh) :TBSRazorBig (Variables|Default|GetRazorMesh)))
  ;[1 1 1] Handle Collision Responses
  (Collision|SetCollisionObjectType (select (== (Utilities|Enum|LiteralenumETBSRazor "TBSClipper") NewToolType) (Utilities|Enum|LiteralenumECollisionChannel "ECC_Vehicle") (Utilities|Enum|LiteralenumECollisionChannel "ECC_Pawn"))))

(fn ConstructionScript)

(fn TrimBeardHair
  (params (StaticMeshComponent :type Primitive%20Component%20Object%20Reference) (Trim%25 :type Float%20%28single-precision%29 :default 0.0))
  (bind _returnvalue (Rendering|Material|CreateDynamicMaterialInstance StaticMeshComponent 0 (Rendering|Material|GetMaterial StaticMeshComponent 0) :!class /Script/Engine.PrimitiveComponent))
  (Rendering|Material|SetScalarParameterValue _returnvalue "Trim%" Trim%25 :!class /Script/Engine.MaterialInstanceDynamic)
  (if (not (== Trim%25 0.0))
    (Collision|SetCollisionResponsetoChannel StaticMeshComponent "ECC_Vehicle" "ECR_Ignore")))