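; Head Blueprint for the barber shop that resets beards when a customer is created.
; CreatedCustomer finds every Beard_02_BP actor and stores each in the Beard variable, an assignment marked for later removal.
; It makes each static mesh component on those beards visible and sets its collision response to overlap all channels.
; Where the first material is a dynamic instance, it zeroes the Trim% scalar parameter.
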(event EventCreatedCustomer
  (bind _outactors (Actor|GetAllActorsOfClass "/Game/TheBarberShop/Assets/Characters/Style_02/Beard_02_BP.Beard_02_BP_C"))
  (for _array_element _outactors
    (bind _asbeard_02_bp (Utilities|Casting|CastToBeard_02_BP _array_element))
    (Variables|Default|SetBeard _asbeard_02_bp) ; -Set For Code Execution\n-to be removed later
    (for _array_element_2 (Actor|GetComponentsByClass _asbeard_02_bp "/Script/Engine.StaticMeshComponent")
      (Utilities|FlowControl|Sequence
        (:then_0
          (Rendering|SetVisibility _array_element_2 true false)
          (Collision|SetCollisionResponsetoAllChannels _array_element_2 "ECR_Overlap"))
        (:then_1
          (bind _asmaterial_instance_dynamic (Utilities|Casting|CastToMaterialInstanceDynamic (Rendering|Material|GetMaterial _array_element_2 0)))
          (Rendering|Material|SetScalarParameterValue _asmaterial_instance_dynamic "Trim%" 0.0 :!class /Script/Engine.MaterialInstanceDynamic))))))

(fn ConstructionScript)