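; Player controller for The Barber Shop that drives the results screen between customers.
; On begin play it attaches the audio listener to the controlled character's camera.
; When a customer is finished it enables the HUD's Results state and mouse cursor, then after a short delay feeds the character's calculated result to the ResultScreen percentage target.
; Spawning the next customer resets that target to zero.
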(event EventSpawnedNextCustomer
  (bind _astbshud_bp (Utilities|Casting|CastToTBSHUD_BP (HUD|GetHUD)))
  (bind _asresult_screen (Utilities|Casting|CastToResultScreen (Variables|/Game/TheBarberShop/Interface/HUD/TBSHUD_BP.TBSHUD_BP_C|GetResultScreen _astbshud_bp)))
  (Variables|/Game/TheBarberShop/Interface/HUD/Ingame/ResultScreen/ResultScreen.ResultScreen_C|SetFloatPercentageTarget _asresult_screen 0.0))

(event EventFinishedCurrentCustomer
  (bind _astbshud (Utilities|Casting|CastToTBSHUD (HUD|GetHUD)))
  (Class|StateComponent|SetState (Variables|/Script/TBS.TBSHUD|GetStateComponent _astbshud) (Utilities|Enum|LiteralenumETBSHUDState "Results") true)
  (Variables|Default|SetbShowMouseCursor true)
  (Utilities|FlowControl|Delay 0 0.5)
  (bind _astbshud_bp (Utilities|Casting|CastToTBSHUD_BP (HUD|GetHUD)))
  (bind _asresult_screen (Utilities|Casting|CastToResultScreen (Variables|/Game/TheBarberShop/Interface/HUD/TBSHUD_BP.TBSHUD_BP_C|GetResultScreen _astbshud_bp)))
  (bind _astbscharacter (Utilities|Casting|CastToTBSCharacter (Pawn|GetControlledPawn)))
  (bind _returnvalue (Class|TBSCharacter|CalculateResult _astbscharacter))
  (Variables|/Game/TheBarberShop/Interface/HUD/Ingame/ResultScreen/ResultScreen.ResultScreen_C|SetFloatPercentageTarget _asresult_screen _returnvalue))

(event EventBeginPlay
  (bind _astbscharacter (Utilities|Casting|CastToTBSCharacter (Pawn|GetControlledPawn)))
  (Class|PlayerController|SetAudioListenerOverride (Variables|/Script/TBS.TBSCharacter|GetCameraComponent _astbscharacter) "0, 0, 0" "0, 0, 0"))

(fn ConstructionScript)