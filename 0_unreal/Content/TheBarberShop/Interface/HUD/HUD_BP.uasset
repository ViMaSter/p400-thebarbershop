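; HUD Blueprint for The Barber Shop that creates the start screen, options, stats, toolbar and beard editor widgets at BeginPlay, starting in the Ingame state.
; Tick pulses the green channel of the stats widget's barber pole material as an example effect.
; Debug keys grant EXP, switch HUD states and print saved beard names.
; Load, save and delete helpers route beard requests to the editor's confirmation dialogs, with only load checking that the name exists.
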(event EventBeginPlay
  (Class|TBSHUD|SetHUDState "Ingame")
  (Utilities|FlowControl|Sequence
    (:then_0
      (bind _returnvalue (UserInterface|CreateWidget "/Game/TheBarberShop/Interface/HUD/StartScreen/StartScreen_MainMenu.StartScreen_MainMenu_C"))
      (bind _output_get (Variables|Default|SetStartScreen _returnvalue))
      (UserInterface|Viewport|AddtoViewport _output_get 0)
      (Input|EnableInput (Game|GetPlayerController 0)))
    (:then_1
      (bind _returnvalue_2 (UserInterface|CreateWidget "/Game/TheBarberShop/Interface/HUD/Options/Options_Menu.Options_Menu_C"))
      (bind _output_get_2 (Variables|Default|SetOptions _returnvalue_2))
      (UserInterface|Viewport|AddtoViewport _output_get_2 0)
      (Input|EnableInput (Game|GetPlayerController 0)))
    (:then_2
      (bind _returnvalue_3 (UserInterface|CreateWidget "/Game/TheBarberShop/Interface/HUD/Options/Options_Audio.Options_Audio_C"))
      (bind _output_get_3 (Variables|Default|SetOptions_Audio _returnvalue_3))
      (UserInterface|Viewport|AddtoViewport _output_get_3 0)
      (Input|EnableInput (Game|GetPlayerController 0)))
    (:then_3
      (bind _returnvalue_4 (UserInterface|CreateWidget "/Game/TheBarberShop/Interface/HUD/Options/Options_Video.Options_Video_C"))
      (bind _output_get_4 (Variables|Default|SetOptions_Video _returnvalue_4))
      (UserInterface|Viewport|AddtoViewport _output_get_4 0)
      (Input|EnableInput (Game|GetPlayerController 0)))
    (:then_4
      (bind _returnvalue_5 (UserInterface|CreateWidget "/Game/TheBarberShop/Interface/HUD/Ingame/Stats/Stats.Stats_C"))
      (bind _output_get_5 (Variables|Default|SetIngame_Stats _returnvalue_5))
      (UserInterface|Viewport|AddtoViewport _output_get_5 0)
      (Input|EnableInput (Game|GetPlayerController 0)))
    (:then_5
      (bind _returnvalue_6 (UserInterface|CreateWidget "/Game/TheBarberShop/Interface/HUD/Ingame/ToolBar/ToolBar.ToolBar_C"))
      (bind _output_get_6 (Variables|Default|SetIngame_Tools _returnvalue_6))
      (UserInterface|Viewport|AddtoViewport _output_get_6 0)
      (Input|EnableInput (Game|GetPlayerController 0)))
    (:then_6
      (bind _returnvalue_7 (UserInterface|CreateWidget "/Game/TheBarberShop/Interface/HUD/Ingame/EditorInterface/EditorInterface.EditorInterface_C"))
      (bind _output_get_7 (Variables|Default|SetEditor _returnvalue_7))
      (UserInterface|Viewport|AddtoViewport _output_get_7 0)
      (Input|EnableInput (Game|GetPlayerController 0)))))

(event EventTick
  (params (DeltaSeconds :type Float%20%28single-precision%29))
  ;[1 1 1] Barber pole material example
  (bind _asstats (Utilities|Casting|CastToStats (Variables|Default|GetIngame_Stats)))
  (Rendering|Material|SetVectorParameterValue (Variables|/Game/TheBarberShop/Interface/HUD/Ingame/Stats/Stats.Stats_C|GetBarberPole_pole_instance _asstats) "Color" (Utilities|Struct|MakeLinearColor 0.0 (+ (/ (Math|Trig|Sin(Degrees) (* (Utilities|Time|GetGameTimeinSeconds) 1e+02)) 2.0) 0.5) 0.0 1.0) :!class /Script/Engine.MaterialInstanceDynamic))

(event Input|KeyboardEvents|F
  ;[1 1 1] HUD-toggling
  (:Pressed
    (Class|TBSHUD|SetHUDState "StartScreen")
    (bind _astbsplayer_controller (Utilities|Casting|CastToTBSPlayerController (Game|GetPlayerController 0)))
    (Variables|/Script/Engine.PlayerController|SetbShowMouseCursor _astbsplayer_controller true)
    (Variables|/Script/TBS.TBSPlayerController|SetInputIgnore _astbsplayer_controller true)))

(event Input|KeyboardEvents|X
  ;[0 0 0] Debugging
  ;;[1 1 1] EXP
  (:Pressed
    (bind _astbscharacter (Utilities|Casting|CastToTBSCharacter (Class|HUD|GetOwningPawn)))
    (Class|TBSCharacter|IncreaseEXP _astbscharacter 10)))

(event Input|KeyboardEvents|Z
  ;[0 0 0] Debugging
  ;;[1 1 1] EXP
  (:Pressed
    (bind _astbscharacter (Utilities|Casting|CastToTBSCharacter (Class|HUD|GetOwningPawn)))
    (Class|TBSCharacter|IncreaseEXP _astbscharacter 1)))

(event Input|KeyboardEvents|C
  ;[0 0 0] Debugging
  ;;[1 1 1] EXP
  (:Pressed
    (bind _astbscharacter (Utilities|Casting|CastToTBSCharacter (Class|HUD|GetOwningPawn)))
    (Class|TBSCharacter|IncreaseEXP _astbscharacter 100)))

(event Input|KeyboardEvents|V
  ;[0 0 0] Debugging
  ;;[1 1 1] EXP
  (:Pressed
    (bind _astbscharacter (Utilities|Casting|CastToTBSCharacter (Class|HUD|GetOwningPawn)))
    (Class|TBSCharacter|IncreaseEXP _astbscharacter 1000)))

(event Input|KeyboardEvents|B
  ;[0 0 0] Debugging
  ;;[1 1 1] EXP
  (:Pressed
    (bind _astbscharacter (Utilities|Casting|CastToTBSCharacter (Class|HUD|GetOwningPawn)))
    (Class|TBSCharacter|IncreaseEXP _astbscharacter 10000)))

(event Input|KeyboardEvents|N
  ;[0 0 0] Debugging
  ;;[1 1 1] EXP
  (:Pressed
    (bind _astbscharacter (Utilities|Casting|CastToTBSCharacter (Class|HUD|GetOwningPawn)))
    (Class|TBSCharacter|IncreaseEXP _astbscharacter 100000)))

(event Input|KeyboardEvents|M
  ;[0 0 0] Debugging
  ;;[1 1 1] EXP
  (:Pressed
    (bind _astbscharacter (Utilities|Casting|CastToTBSCharacter (Class|HUD|GetOwningPawn)))
    (Class|TBSCharacter|IncreaseEXP _astbscharacter 1000000)))

(event Input|KeyboardEvents|E
  ;[1 1 1] HUD-toggling
  (:Pressed
    (bind _aseditor_interface (Utilities|Casting|CastToEditorInterface (Variables|Default|GetEditor)))
    (Default|RefreshList _aseditor_interface)
    (Class|TBSHUD|ToggleHUDState "Editor")))

(event Input|KeyboardEvents|T
  ;[1 1 1] Debug all currently saved beards
  (:Pressed
    (bind _astbsplayer_controller (Utilities|Casting|CastToTBSPlayerController (Game|GetPlayerController 0)))
    (bind _returnvalue (Class|TBSPlayerController|GetBeardNames _astbsplayer_controller))
    (for _array_element _returnvalue
      (Development|PrintString (Utilities|String|Append "Test: " (Utilities|String|ToString(Name) _array_element))))))

(event Input|KeyboardEvents|G
  ;[1 1 1] HUD-toggling
  (:Pressed
    (Class|TBSHUD|SetHUDState "Ingame")))

(fn ConstructionScript)

(fn TryLoadBeard
  (params (BeardName :type Name :default "None"))
  ;[1 1 1] Check whether or not the beard exists
  (bind _astbsplayer_controller (Utilities|Casting|CastToTBSPlayerController (Game|GetPlayerController 0)))
  (bind _returnvalue (Class|TBSPlayerController|GetBeardNames _astbsplayer_controller))
  (if (Utilities|Array|ContainsItem _returnvalue BeardName)
    ;[1 1 1] Open Confirmation-Dialog if so
    (bind _aseditor_interface (Utilities|Casting|CastToEditorInterface (Variables|Default|GetEditor)))
    (Default|ChangeBeardtoLoad _aseditor_interface BeardName false)
    (LocalVariables|SetisSuccess true)
    (else
      (LocalVariables|SetisSuccess false)))
  (return (LocalVariables|GetisSuccess)))

(fn TrySaveBeard
  (params (BeardName :type Name :default "None"))
  ;[1 1 1] Open Confirmation-Dialog if so
  (bind _aseditor_interface (Utilities|Casting|CastToEditorInterface (Variables|Default|GetEditor)))
  (Default|ChangeBeardtoSave _aseditor_interface BeardName false))

(fn TryDeleteBeard
  (params (BeardName :type Name :default "None"))
  ;[1 1 1] Open Confirmation-Dialog if so
  (bind _aseditor_interface (Utilities|Casting|CastToEditorInterface (Variables|Default|GetEditor)))
  (Default|ChangeBeardtoDelete _aseditor_interface BeardName false))