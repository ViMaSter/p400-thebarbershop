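; HUD Blueprint for TheBarberShop that sets up the main menu and options screens.
; On BeginPlay it creates and stores the start screen, options, audio and video widgets, adding all four to the viewport at the same Z-order and enabling player input.
; The F and G keys call SetHUDState to switch to the StartScreen and Intro states, with no switching logic in these graphs.
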(event EventBeginPlay
  (Utilities|FlowControl|Sequence
    (:then_0
      (bind _returnvalue (UserInterface|CreateWidget "/Game/TheBarberShop/Blueprints/HUD/StartScreen/StartScreen_MainMenu.StartScreen_MainMenu_C"))
      (bind _output_get (Variables|Default|SetStartScreen _returnvalue))
      (UserInterface|Viewport|AddtoViewport _output_get 0)
      (Input|EnableInput (Game|GetPlayerController 0)))
    (:then_1
      (bind _returnvalue_2 (UserInterface|CreateWidget "/Game/TheBarberShop/Blueprints/HUD/Options/Options_Menu.Options_Menu_C"))
      (bind _output_get_2 (Variables|Default|SetOptions _returnvalue_2))
      (UserInterface|Viewport|AddtoViewport _output_get_2 0)
      (Input|EnableInput (Game|GetPlayerController 0)))
    (:then_2
      (bind _returnvalue_3 (UserInterface|CreateWidget "/Game/TheBarberShop/Blueprints/HUD/Options/Options_Audio.Options_Audio_C"))
      (bind _output_get_3 (Variables|Default|SetOptions_Audio _returnvalue_3))
      (UserInterface|Viewport|AddtoViewport _output_get_3 0)
      (Input|EnableInput (Game|GetPlayerController 0)))
    (:then_3
      (bind _returnvalue_4 (UserInterface|CreateWidget "/Game/TheBarberShop/Blueprints/HUD/Options/Options_Video.Options_Video_C"))
      (bind _output_get_4 (Variables|Default|SetOptions_Video _returnvalue_4))
      (UserInterface|Viewport|AddtoViewport _output_get_4 0)
      (Input|EnableInput (Game|GetPlayerController 0)))))

(event Input|KeyboardEvents|F
  (:Pressed
    (Class|TBSHUD|SetHUDState "StartScreen")))

(event Input|KeyboardEvents|G
  (:Pressed
    (Class|TBSHUD|SetHUDState "Intro")))

(fn ConstructionScript)